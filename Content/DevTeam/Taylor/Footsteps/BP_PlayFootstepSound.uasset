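; Anim notify that plays a skeleton footstep sound, with enemy footstep attenuation, on the animated mesh.
; When fired, it traces straight down from the owning actor on the Visibility channel and plays the sound only if something is hit.
; Volume scales with the owner's speed through a clamped range map, and the hit surface does not affect which sound plays.
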(fn `Received_Notify`
  (params (MeshComp :type "SkeletalMeshComponent Object Reference") (Animation :type "AnimSequenceBase Object Reference") (EventReference :type "AnimNotifyEventReference Structure (by ref)"))
  (returns (ReturnValue :type Boolean))
  (bind _returnvalue (`ActorComponent.GetOwner` MeshComp))
  (bind _returnvalue_2 (`Actor.K2_GetActorLocation` _returnvalue))
  (bind (_outhit _returnvalue_3) (`KismetSystemLibrary.LineTraceSingle` _returnvalue_2 (`KismetMathLibrary.MakeVector` (.x _returnvalue_2) (.y _returnvalue_2) (- (.z _returnvalue_2) 500.0)) "TraceTypeQuery1" false (`|MakeArray` _returnvalue)))
  (if _returnvalue_3
    (`GameplayStatics.SpawnSoundAttached` "/Game/DevTeam/Taylor/Sounds/SkeletonStep.SkeletonStep" (`local.MeshComp`) "None" (0.0 0.0 0.0) (struct) "KeepRelativeOffset" false (`KismetMathLibrary.MapRangeClamped` (`KismetMathLibrary.VSize` (`Actor.GetVelocity` _returnvalue)) 0.0 600.0 0.0 1.5) 1.0 0.0 "/Game/DevTeam/Taylor/Footsteps/SA_EnemyFootsteps.SA_EnemyFootsteps" null)
    (return false)
    (else
      (return false))))