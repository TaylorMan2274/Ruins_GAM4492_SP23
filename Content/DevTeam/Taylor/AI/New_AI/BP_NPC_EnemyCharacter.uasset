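; Enemy NPC character that carries its own spline movement path and changes walk speed with its alert state.
; BeginPlay detaches the path, keeping its world transform, and the construction script closes the spline loop when PathIsClosedLoop is set.
; The AlertState event stores the state and, through a DoOnce that ResetAlert immediately re-arms, sets a slower speed for Neutral and a faster one for Alert.
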(event `self.ReceiveBeginPlay`
  (`SceneComponent.K2_DetachFromComponent` (`self.MovementPath`) "KeepWorld" "KeepWorld" "KeepWorld" true))

(event `/Game/DevTeam/Taylor/AI/New_AI/BPI_NPC.AlertState`
  (params (`Alert State` :type "/Game/DevTeam/Taylor/AI/New_AI/Enum_AlertState Enum" :default "NewEnumerator0"))
  (set `self.Alert State` `Alert State`)
  (`/Engine/EditorBlueprintResources/StandardMacros.DoOnce` false :!label _label
    (:`Completed`
      (set `CharacterMovementComponent.MaxWalkSpeed` (select `/Game/DevTeam/Taylor/AI/New_AI/Enum_AlertState` (`self.Alert State`) :`NewEnumerator0` 250.0 :`NewEnumerator1` 750.0 :!type "Float (single-precision)") (`self.CharacterMovement`))
      (`self.ResetAlert`))))

(event `ResetAlert`
  (goto _label :!via `Reset`))

(fn `UserConstructionScript`
  (if (`self.PathIsClosedLoop`)
    (`SplineComponent.SetClosedLoop` (`self.MovementPath`) true true)))