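; BP_EnemyController is the AI controller for enemy characters, driving patrol and player detection through the BT_Enemy behavior tree.
; On BeginPlay it runs the tree, caches the BP_EnemyCharacter pawn and seeds the blackboard with its patrol path's looping flag and wait time, plus an initial direction.
; AI Perception updates set CanSeePlayer from the sensed result, only for BP_ThirdPersonCharacter actors.
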(event `self.ReceiveBeginPlay`
  (`self.RunBehaviorTree` "/Game/DevTeam/Taylor/AI/BT_Enemy.BT_Enemy")
  (bind _asbp_enemy_character (cast `/Game/DevTeam/Taylor/AI/BP_EnemyCharacter` (`self.K2_GetPawn`)))
  (bind _output_get (set `self.MyPawn` _asbp_enemy_character))
  (`BlackboardComponent.SetValueAsBool` (`self.Blackboard`) (`self.PathLooping`) (`/Game/DevTeam/Taylor/AI/BP_PatrolPath.IsLooping` (`/Game/DevTeam/Taylor/AI/BP_EnemyCharacter.PatrolPath` _output_get)))
  (`BlackboardComponent.SetValueAsInt` (`self.Blackboard`) (`self.Direction`) 1)
  (`BlackboardComponent.SetValueAsFloat` (`self.Blackboard`) (`self.WaitTime`) (`/Game/DevTeam/Taylor/AI/BP_PatrolPath.WaitTime` (`/Game/DevTeam/Taylor/AI/BP_EnemyCharacter.PatrolPath` (`self.MyPawn`)))))

(event `self.AIPerception.OnTargetPerceptionUpdated`
  (params (Actor :type "Actor Object Reference") (Stimulus :type "AIStimulus Structure"))
  (cast `/Game/ThirdPerson/Blueprints/BP_ThirdPersonCharacter` Actor)
  (`BlackboardComponent.SetValueAsBool` (`self.Blackboard`) (`self.CanSeePlayer`) (`.bSuccessfullySensed` (break `AIStimulus` Stimulus))))

(fn `UserConstructionScript`)