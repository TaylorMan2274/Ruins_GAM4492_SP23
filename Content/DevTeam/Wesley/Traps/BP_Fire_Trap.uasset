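; BP_Fire_Trap is a trap that cycles its fire on and off and damages the player.
; A looping timer drives a FlipFlop that toggles the fire, its audio and the FireDamage flag.
; Damage hits Hunter_Bp2 when fire ignites on an overlapping player or the player enters the damage box while lit.
; CanTakeDamage resets after a delay but is never checked, and the Pendulum reference is unused.
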(event `self.ReceiveBeginPlay`
  (`KismetSystemLibrary.K2_SetTimerDelegate` (delegate `FireActivate-Deactivate`) (`self.Time`) true)
  (bind _returnvalue (`GameplayStatics.GetActorOfClass` "/Game/DevTeam/Deon/Pendulum.Pendulum_C"))
  (set `self.pend ref` _returnvalue))

(event `FireIsActivate`)

(event `FireActivate-Deactivate`
  (bind _fire (`self.Fire`))
  (`/Engine/EditorBlueprintResources/StandardMacros.FlipFlop`
    (:`A`
      (`ActorComponent.Deactivate` _fire)
      (`ActorComponent.Deactivate` (`self.FireAudio`))
      (set `self.Fire Damage?` false))
    (:`B`
      (`ActorComponent.Activate` _fire true)
      (`ActorComponent.Activate` (`self.FireAudio`) true)
      (set `self.Fire Damage?` true)
      (for _array_element (`self.GetOverlappingActors` null)
        (if (== _array_element (`GameplayStatics.GetPlayerCharacter` 0))
          (set `self.CanTakeDamage` false :!label _label)
          (bind _ashunter_bp_2 (cast `/Game/DevTeam/Rick/Hunter_Bp2` (`GameplayStatics.GetPlayerCharacter` 0)))
          (`/Game/DevTeam/Rick/Hunter_Bp2.Take damage` _ashunter_bp_2 (`self.MyDamage`))
          (`KismetSystemLibrary.Delay` 1.0)
          (set `self.CanTakeDamage` true))))))

(event `self.ReceiveTick`
  (params (DeltaSeconds :type "Float (single-precision)")))

(event `self.Coll_BoxDamage.OnComponentBeginOverlap`
  (params (OverlappedComponent :type "PrimitiveComponent Object Reference") (OtherActor :type "Actor Object Reference") (OtherComp :type "PrimitiveComponent Object Reference") (OtherBodyIndex :type Integer) (bFromSweep :type Boolean) (SweepResult :type "HitResult Structure (by ref)"))
  (if (`self.Fire Damage?`)
    (if (== OtherActor (`GameplayStatics.GetPlayerCharacter` 0))
      (if true
        (goto _label)))))

(event `self.Coll_BoxDamage.OnComponentEndOverlap`
  (params (OverlappedComponent :type "PrimitiveComponent Object Reference") (OtherActor :type "Actor Object Reference") (OtherComp :type "PrimitiveComponent Object Reference") (OtherBodyIndex :type Integer)))

(fn `Fire Damage`)

(fn `UserConstructionScript`)