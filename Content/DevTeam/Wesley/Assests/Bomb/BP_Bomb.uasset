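; BP_Bomb is a bomb pickup actor that the player collects by interacting with it.
; BeginPlay creates an interact prompt widget and a bomb-picked-up widget.
; The Coll_Box overlap events show and hide the prompt for the player character only.
; Interact destroys the actor and then adds the picked-up widget to the viewport, without checking overlap or recording the pickup.
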(event `self.ReceiveBeginPlay`
  (bind _returnvalue (`|CreateWidget` "/Game/DevTeam/Wesley/BP_Interactions/P_Interact.P_Interact_C"))
  (set `self.Interact Prompt` _returnvalue)
  (bind _returnvalue_2 (`|CreateWidget` "/Game/DevTeam/Wesley/BP_Interactions/P_BombPickedup.P_BombPickedup_C"))
  (set `self.Bomb Picked up` _returnvalue_2))

(event `self.Coll_Box.OnComponentBeginOverlap`
  (params (OverlappedComponent :type "PrimitiveComponent Object Reference") (OtherActor :type "Actor Object Reference") (OtherComp :type "PrimitiveComponent Object Reference") (OtherBodyIndex :type Integer) (bFromSweep :type Boolean) (SweepResult :type "HitResult Structure (by ref)"))
  (if (== OtherActor (`GameplayStatics.GetPlayerCharacter` 0))
    (`UserWidget.AddToViewport` (`self.Interact Prompt`) 0)))

(event `self.Coll_Box.OnComponentEndOverlap`
  (params (OverlappedComponent :type "PrimitiveComponent Object Reference") (OtherActor :type "Actor Object Reference") (OtherComp :type "PrimitiveComponent Object Reference") (OtherBodyIndex :type Integer))
  (if (== (`GameplayStatics.GetPlayerCharacter` 0) OtherActor)
    (`Widget.RemoveFromParent` (`self.Interact Prompt`))))

(event `/Game/DevTeam/Wesley/BP_Interactions/InteractInterface.Interact`
  (`self.K2_DestroyActor`)
  (`UserWidget.AddToViewport` (`self.Bomb Picked up`) 0))

(fn `UserConstructionScript`)