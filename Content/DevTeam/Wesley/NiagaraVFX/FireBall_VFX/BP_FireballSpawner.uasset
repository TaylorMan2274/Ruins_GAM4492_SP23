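; BP_FireballSpawner is an actor that repeatedly launches BP_FireBall actors into the level.
; A looping two-second timer started on BeginPlay spawns each fireball at the transform of an Arrow component.
; The sphere hit event is empty, and a disconnected branch holds unused spawn logic that depends on player yaw.
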(event `self.ReceiveBeginPlay`
  (`KismetSystemLibrary.K2_SetTimerDelegate` (delegate `SpawnFireBall`) 2.0 true))

(event `SpawnFireBall`
  (bind (_returnvalue_location _returnvalue_rotation _returnvalue_scale) (`KismetMathLibrary.BreakTransform` (`SceneComponent.K2_GetComponentToWorld` (`self.Arrow`))))
  (`|SpawnActorFromClass` "/Game/DevTeam/Wesley/NiagaraVFX/FireBall_VFX/BP_FireBall.BP_FireBall_C" (`KismetMathLibrary.MakeTransform` _returnvalue_location _returnvalue_rotation _returnvalue_scale) "Undefined" "OverrideRootScale" null 1000.0 (0.0 1.0 0.0) null))

(event `self.Sphere.OnComponentHit`
  (params (HitComponent :type "PrimitiveComponent Object Reference") (OtherActor :type "Actor Object Reference") (OtherComp :type "PrimitiveComponent Object Reference") (NormalImpulse :type "Vector Structure") (Hit :type "HitResult Structure (by ref)")))

(fn `UserConstructionScript`)