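; BP_FireBall is a projectile actor, launched on BeginPlay by a velocity-change impulse along Direction scaled by Intensity.
; Capsule hits on BP_NPC_EnemyCharacter deactivate movement and play a dizzy montage, with restoration queued behind a short Delay.
; Hits on the player attach a burn Niagara effect and apply damage.
; Every hit also spawns an explosion and destroys the fireball immediately, before that Delay can finish.
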(event `self.ReceiveBeginPlay`
  (`PrimitiveComponent.AddImpulse` (`self.Coll_Capsule`) (* (`self.Intensity`) (`self.Direction`)) "None" true))

(event `self.Fireball.OnComponentHit`
  (params (HitComponent :type "PrimitiveComponent Object Reference") (OtherActor :type "Actor Object Reference") (OtherComp :type "PrimitiveComponent Object Reference") (NormalImpulse :type "Vector Structure") (Hit :type "HitResult Structure (by ref)")))

(event `self.Coll_Capsule.OnComponentHit`
  (params (HitComponent :type "PrimitiveComponent Object Reference") (OtherActor :type "Actor Object Reference") (OtherComp :type "PrimitiveComponent Object Reference") (NormalImpulse :type "Vector Structure") (Hit :type "HitResult Structure (by ref)"))
  (`|ExecutionSequence`
    (:`then_0`
      (if (`KismetStringLibrary.Contains` (`KismetSystemLibrary.GetDisplayName` OtherActor) "BP_NPC_EnemyCharacter")
        (bind _asbp_npc_enemy_character (cast `/Game/DevTeam/Taylor/AI/New_AI/BP_NPC_EnemyCharacter` OtherActor))
        (`ActorComponent.Deactivate` (`Character.CharacterMovement` _asbp_npc_enemy_character))
        (`Character.PlayAnimMontage` _asbp_npc_enemy_character "/Game/DevTeam/Rick/sk_bp/skdizzy_Montage.skdizzy_Montage" 1.0 "None")
        (`KismetSystemLibrary.Delay` 0.25)
        (`Character.StopAnimMontage` _asbp_npc_enemy_character "/Game/DevTeam/Rick/sk_bp/skdizzy_Montage.skdizzy_Montage")
        (`ActorComponent.Activate` (`Character.CharacterMovement` _asbp_npc_enemy_character) false)))
    (:`then_1`
      (if (== OtherActor (`GameplayStatics.GetPlayerCharacter` 0))
        (bind _ashunter_bp_2 (cast `/Game/DevTeam/Rick/Hunter_Bp2` OtherActor))
        (`NiagaraFunctionLibrary.SpawnSystemAttached` "/Game/DevTeam/Wesley/NiagaraVFX/NS_HunterBurn_Base.NS_HunterBurn_Base" (`Character.Mesh` _ashunter_bp_2) "None" (0.0 0.0 0.0) (struct) "KeepRelativeOffset")
        (`GameplayStatics.ApplyDamage` OtherActor (`self.Base Damage`)))
      (`NiagaraFunctionLibrary.SpawnSystemAtLocation` "/Game/DevTeam/Wesley/NiagaraVFX/FireBall_VFX/NS_Explosion_Base.NS_Explosion_Base" (`SceneComponent.K2_GetComponentLocation` (`self.Fireball`)))
      (`self.K2_DestroyActor`))))

(fn `UserConstructionScript`)