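; Test smasher trap that slowly raises a cube, slams it back down and damages the hunter character.
; A self-restarting Start event, kicked off on BeginPlay, waits a configurable delay, raises the cube, pauses, then drops it quickly.
; Rise and Fall helpers derive each target by offsetting the cube's current relative Z.
; A Box overlap casts to Hunter_Bp2 and applies Damage, independent of the movement phase.
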(event `Start`
  (bind _cube (`self.Cube`))
  (bind _cube_2 (`self.Cube`))
  (`KismetSystemLibrary.Delay` (`self.Startdelay`))
  (bind _location (`self.Rise` _cube_2))
  (`KismetSystemLibrary.MoveComponentTo` _cube_2 _location (struct) false false 5.0)
  (`KismetSystemLibrary.Delay` 2.0)
  (bind _location_2 (`self.fall` _cube))
  (`KismetSystemLibrary.MoveComponentTo` _cube _location_2 (struct) false false 0.5)
  (`self.Start`))

(event `self.ReceiveBeginPlay`
  (`self.Start`))

(event `self.Box.OnComponentBeginOverlap`
  (params (OverlappedComponent :type "PrimitiveComponent Object Reference") (OtherActor :type "Actor Object Reference") (OtherComp :type "PrimitiveComponent Object Reference") (OtherBodyIndex :type Integer) (bFromSweep :type Boolean) (SweepResult :type "HitResult Structure (by ref)"))
  (bind _ashunter_bp_2 (cast `/Game/DevTeam/Rick/Hunter_Bp2` OtherActor))
  (`/Game/DevTeam/Rick/Hunter_Bp2.Take damage` _ashunter_bp_2 (`self.Damage`)))

(fn `fall`
  (params (sm :type "StaticMeshComponent Object Reference"))
  (returns (location :type "Vector Structure"))
  (bind (_relativelocation_x _relativelocation_y _relativelocation_z) (`KismetMathLibrary.BreakVector` (`SceneComponent.RelativeLocation` sm)))
  (return (`KismetMathLibrary.MakeVector` _relativelocation_x _relativelocation_y (+ _relativelocation_z -300.0))))

(fn `Rise`
  (params (sm :type "StaticMeshComponent Object Reference"))
  (returns (location :type "Vector Structure"))
  (bind (_relativelocation_x _relativelocation_y _relativelocation_z) (`KismetMathLibrary.BreakVector` (`SceneComponent.RelativeLocation` sm)))
  (return (`KismetMathLibrary.MakeVector` _relativelocation_x _relativelocation_y (+ _relativelocation_z 300.0))))

(fn `UserConstructionScript`)