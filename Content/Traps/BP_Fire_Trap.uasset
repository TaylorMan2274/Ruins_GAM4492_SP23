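; BP_Fire_Trap is a trap whose Fire component switches on and off on a looping timer started at BeginPlay.
; A FlipFlop alternates deactivating and activating Fire on each timer tick.
; Coll_BoxDamage overlaps set and clear a FireDamage flag with debug prints, while Coll_BoxNoDamage clears it on entry.
; No damage is applied: the Fire Damage function is empty, and the flag is independent of the fire's state.
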(event `self.ReceiveBeginPlay`
  (`KismetSystemLibrary.K2_SetTimerDelegate` (delegate `FireActivate-Deactivate`) 5.0 true))

(event `FireIsActivate`)

(event `FireActivate-Deactivate`
  (bind _fire (`self.Fire`))
  (`/Engine/EditorBlueprintResources/StandardMacros.FlipFlop`
    (:`A`
      (`ActorComponent.Deactivate` _fire))
    (:`B`
      (`ActorComponent.Activate` _fire true))))

(event `self.ReceiveTick`
  (params (DeltaSeconds :type "Float (single-precision)")))

(event `self.Coll_BoxDamage.OnComponentBeginOverlap`
  (params (OverlappedComponent :type "PrimitiveComponent Object Reference") (OtherActor :type "Actor Object Reference") (OtherComp :type "PrimitiveComponent Object Reference") (OtherBodyIndex :type Integer) (bFromSweep :type Boolean) (SweepResult :type "HitResult Structure (by ref)"))
  (set `self.Fire Damage?` true)
  (`KismetSystemLibrary.PrintString` "Hello1"))

(event `self.Coll_BoxDamage.OnComponentEndOverlap`
  (params (OverlappedComponent :type "PrimitiveComponent Object Reference") (OtherActor :type "Actor Object Reference") (OtherComp :type "PrimitiveComponent Object Reference") (OtherBodyIndex :type Integer))
  (set `self.Fire Damage?` false)
  (`KismetSystemLibrary.PrintString` "Hello2"))

(event `self.Coll_BoxNoDamage.OnComponentBeginOverlap`
  (params (OverlappedComponent :type "PrimitiveComponent Object Reference") (OtherActor :type "Actor Object Reference") (OtherComp :type "PrimitiveComponent Object Reference") (OtherBodyIndex :type Integer) (bFromSweep :type Boolean) (SweepResult :type "HitResult Structure (by ref)"))
  (set `self.Fire Damage?` false)
  (if (`self.Fire Damage?`)
    (`KismetSystemLibrary.PrintText` "Hello")))

(fn `Fire Damage`)

(fn `UserConstructionScript`)